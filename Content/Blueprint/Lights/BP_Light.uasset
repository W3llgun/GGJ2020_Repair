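; BP_Light is a toggleable light actor with a spotlight, an emissive mesh and a light shaft cone.
; The construction script applies LightColor to the spotlight and to dynamic material instances on the mesh and shaft.
; ToggleLight flips State, then sets spotlight visibility including its children, emissive intensity and actor collision to match.
; BeginPlay applies the initial State without flipping it, and the shaft's overlap event is empty.
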(event OnComponentBeginOverlap(SM_Lightshaft_cyl)
  (params (OverlappedComponent :type Primitive%20Component%20Object%20Reference) (OtherActor :type Actor%20Object%20Reference) (OtherComp :type Primitive%20Component%20Object%20Reference) (OtherBodyIndex :type Integer) (bFromSweep :type Boolean) (SweepResult :type Hit%20Result%20Structure%20%28by%20ref%29)))

(event EventBeginPlay
  (bind _spotlight (Variables|Default|GetSpotLight))
  ;[1 1 1] ToggleLight
  (if (Variables|Default|GetbState)
    (Development|SetHiddeninGame _spotlight false true)
    (else
      (Development|SetHiddeninGame _spotlight true true)))
  (bind _returnvalue (Rendering|Material|CreateDynamicMaterialInstance (Variables|Default|GetCube) 0 "/Game/Geometry/Materials/MI_Emiss_01.MI_Emiss_01" "None" :!class /Script/Engine.PrimitiveComponent))
  (bind _returnvalue_2 (Rendering|Material|GetScalarParameterValue _returnvalue "EmissIntensity" :!class /Script/Engine.MaterialInstanceDynamic))
  (bind _output_get (Variables|Default|SetEmiss_Instance _returnvalue))
  (Rendering|Material|SetScalarParameterValue _output_get "EmissIntensity" (select (Variables|Default|GetbState) _returnvalue_2 0.0) :!class /Script/Engine.MaterialInstanceDynamic)
  (Collision|SetActorEnableCollision (Variables|Default|GetbState)))

(event EventToggleLight
  (bind _spotlight (Variables|Default|GetSpotLight))
  ;[1 1 1] ToggleLight
  (Variables|Default|SetbState (not (Variables|Default|GetbState)))
  (if (Variables|Default|GetbState)
    (Development|SetHiddeninGame _spotlight false true)
    (else
      (Development|SetHiddeninGame _spotlight true true)))
  (bind _returnvalue (Rendering|Material|CreateDynamicMaterialInstance (Variables|Default|GetCube) 0 "/Game/Geometry/Materials/MI_Emiss_01.MI_Emiss_01" "None" :!class /Script/Engine.PrimitiveComponent))
  (bind _returnvalue_2 (Rendering|Material|GetScalarParameterValue _returnvalue "EmissIntensity" :!class /Script/Engine.MaterialInstanceDynamic))
  (bind _output_get (Variables|Default|SetEmiss_Instance _returnvalue))
  (Rendering|Material|SetScalarParameterValue _output_get "EmissIntensity" (select (Variables|Default|GetbState) _returnvalue_2 0.0) :!class /Script/Engine.MaterialInstanceDynamic)
  (Collision|SetActorEnableCollision (Variables|Default|GetbState)))

(fn ConstructionScript
  (bind _lightcolor (Variables|Default|GetLightColor))
  (Rendering|Components|Light|SetLightColor (Variables|Default|GetSpotLight) _lightcolor true)
  (bind _returnvalue (Rendering|Material|CreateDynamicMaterialInstance (Variables|Default|GetCube) 0 "/Game/Geometry/Materials/MI_Emiss_01.MI_Emiss_01" "None" :!class /Script/Engine.PrimitiveComponent))
  (bind _output_get (Variables|Default|SetEmiss_Instance _returnvalue))
  (Rendering|Material|SetVectorParameterValue _output_get "Emiss" _lightcolor :!class /Script/Engine.MaterialInstanceDynamic)
  (bind _returnvalue_2 (Rendering|Material|CreateDynamicMaterialInstance (Variables|Default|GetSM_Lightshaft_cyl) 0 "/Game/Geometry/Materials/MI_LightShaft_01.MI_LightShaft_01" "None" :!class /Script/Engine.PrimitiveComponent))
  (bind _output_get_2 (Variables|Default|SetCone_Color_Instance _returnvalue_2))
  (Rendering|Material|SetVectorParameterValue _output_get_2 "Color" (Variables|Default|GetLightColor) :!class /Script/Engine.MaterialInstanceDynamic))