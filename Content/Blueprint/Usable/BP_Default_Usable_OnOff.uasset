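; Usable actor that switches its linked actors on or off when triggered.
; On TriggerStart it runs the parent logic, then loops through LinkedActors, calling ToggleLight on each BP_Light with a debug print.
; Other actors get their collision flipped, then hidden-in-game and tick are both set to the inverse of the new collision state, so ticking is enabled while hidden.
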(event EventBeginPlay
  (|CallParentFunction) ; This node is disabled and will not be called.\nDrag off pins to build functionality.
)

(event Collision|EventActorBeginOverlap
  (params (OtherActor :type Actor%20Object%20Reference))
  (|CallParentFunction OtherActor) ; This node is disabled and will not be called.\nDrag off pins to build functionality.
)

(event EventTick
  (params (DeltaSeconds :type Float%20%28single-precision%29))
  (|CallParentFunction DeltaSeconds) ; This node is disabled and will not be called.\nDrag off pins to build functionality.
)

(event EventTriggerStart
  (|CallParentFunction)
  (for _array_element (Variables|Default|GetLinkedActors)
    (bind _asbp_light (Utilities|Casting|CastToBP_Light _array_element)
      (:then
        (Default|ToggleLight _asbp_light)
        (Development|PrintString "IsLight"))
      (:CastFailed
        (bind _asactor (Utilities|Casting|CastToActor _array_element))
        (Collision|SetActorEnableCollision _asactor (not (Collision|GetActorEnableCollision _asactor)))
        (Rendering|SetActorHiddenInGame _asactor (not (Collision|GetActorEnableCollision _asactor)))
        (Actor|Tick|SetActorTickEnabled _asactor (not (Collision|GetActorEnableCollision _asactor)))))))

(fn ConstructionScript
  (|CallParentFunction))