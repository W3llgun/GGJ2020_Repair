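; Usable Blueprint that swings a linked actor back and forth between the rotations of two reference actors, Position1 and Position2.
; TriggerStart and TriggerStop toggle movement, and Tick advances a local clock only while enabled, so motion resumes where it paused.
; A speed-scaled sine of that clock drives a shortest-path rotator lerp.
; BeginPlay tints the mesh's emissive material with the default color, while RefreshLight is empty.
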(event EventBeginPlay
  (|CallParentFunction)
  (Utilities|FlowControl|Sequence
    (:then_0
      ;[1 1 1] SetDefaultColor
      (bind _returnvalue (Rendering|Material|CreateDynamicMaterialInstance (Variables|Default|GetStaticMesh) 1 "/Game/Geometry/Materials/MI_Emiss_01.MI_Emiss_01" "None" :!class /Script/Engine.PrimitiveComponent))
      (Rendering|Material|SetVectorParameterValue _returnvalue "Emiss" (Math|Conversions|ToLinearColor(Color) (Variables|Default|GetDefaultColor)) :!class /Script/Engine.MaterialInstanceDynamic))
    (:then_1
      (Variables|Default|SetLocalTime (+ (Variables|Default|GetLocalTime) (stale EventTick DeltaSeconds)))
      (Transformation|SetActorRotation (Variables|Default|GetLinkedActor) (Math|Rotator|Lerp(Rotator) (Transformation|GetActorRotation (Variables|Default|GetPosition1)) (Transformation|GetActorRotation (Variables|Default|GetPosition2)) (* (+ (Math|Trig|Sin(Degrees) (* (Math|Trig|GetPI) (Variables|Default|GetMovementSpeed) 2.0 (Variables|Default|GetLocalTime))) 1.0) 0.5) true)))))

(event Collision|EventActorBeginOverlap
  (params (OtherActor :type Actor%20Object%20Reference))
  (|CallParentFunction OtherActor) ; This node is disabled and will not be called.\nDrag off pins to build functionality.
)

(event EventTick
  (params (DeltaSeconds :type Float%20%28single-precision%29))
  (|CallParentFunction DeltaSeconds)
  (if (Variables|Default|GetAllowMovement)
    (Variables|Default|SetLocalTime (+ (Variables|Default|GetLocalTime) DeltaSeconds))
    (Transformation|SetActorRotation (Variables|Default|GetLinkedActor) (Math|Rotator|Lerp(Rotator) (Transformation|GetActorRotation (Variables|Default|GetPosition1)) (Transformation|GetActorRotation (Variables|Default|GetPosition2)) (* (+ (Math|Trig|Sin(Degrees) (* (Math|Trig|GetPI) (Variables|Default|GetMovementSpeed) 2.0 (Variables|Default|GetLocalTime))) 1.0) 0.5) true))))

(event EventTriggerStart
  (Variables|Default|SetAllowMovement true)
  (|CallParentFunction))

(event EventTriggerStop
  (Variables|Default|SetAllowMovement false))

(event EventRefreshLight)

(fn ConstructionScript
  (|CallParentFunction))