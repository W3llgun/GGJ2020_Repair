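; Usable Blueprint that moves a linked actor back and forth between two position actors while triggered.
; TriggerStart and TriggerStop toggle movement, and Tick advances a local timer only while it is enabled, so motion pauses in place.
; A degree-based sine of time and MovementSpeed, remapped to 0–1, drives the location lerp, which BeginPlay also runs once.
; TriggerStop does not call its parent, unlike TriggerStart.
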(event EventBeginPlay
  (|CallParentFunction)
  (Variables|Default|SetLocalTime (+ (Variables|Default|GetLocalTime) (stale EventTick DeltaSeconds)))
  (Transformation|SetActorLocation (Variables|Default|GetLinkedActor) (Math|Vector|Lerp(Vector) (Transformation|GetActorLocation (Variables|Default|GetPosition1)) (Transformation|GetActorLocation (Variables|Default|GetPosition2)) (* (+ (Math|Trig|Sin(Degrees) (* (Math|Trig|GetPI) (Variables|Default|GetMovementSpeed) 2.0 (Variables|Default|GetLocalTime))) 1.0) 0.5)) false false))

(event Collision|EventActorBeginOverlap
  (params (OtherActor :type Actor%20Object%20Reference))
  (|CallParentFunction OtherActor) ; This node is disabled and will not be called.\nDrag off pins to build functionality.
)

(event EventTick
  (params (DeltaSeconds :type Float%20%28single-precision%29))
  (|CallParentFunction DeltaSeconds)
  (if (Variables|Default|GetAllowMovement)
    (Variables|Default|SetLocalTime (+ (Variables|Default|GetLocalTime) DeltaSeconds))
    (Transformation|SetActorLocation (Variables|Default|GetLinkedActor) (Math|Vector|Lerp(Vector) (Transformation|GetActorLocation (Variables|Default|GetPosition1)) (Transformation|GetActorLocation (Variables|Default|GetPosition2)) (* (+ (Math|Trig|Sin(Degrees) (* (Math|Trig|GetPI) (Variables|Default|GetMovementSpeed) 2.0 (Variables|Default|GetLocalTime))) 1.0) 0.5)) false false)))

(event EventTriggerStart
  (Variables|Default|SetAllowMovement true)
  (|CallParentFunction))

(event EventTriggerStop
  (Variables|Default|SetAllowMovement false))

(fn ConstructionScript
  (|CallParentFunction))