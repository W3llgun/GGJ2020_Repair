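; BP_SwitchCharacter is a transitional actor that carries out a character switch by flying to the destination pawn's camera.
; On spawn it plays a swoosh sound and animates its skeletal mesh scale through a timeline.
; GiveDestination caches the target camera's transform, which Tick interpolates toward.
; When close, it unpossesses the current pawn, destroys itself, possesses the destination and restores that pawn's CustomTimeDilation to normal.
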(event EventBeginPlay
  (bind _skeletalmesh (Variables|Default|GetSkeletalMesh))
  (Audio|PlaySound2D "/Game/Audio/SC_swoosh.SC_swoosh" 1.0 1.0 0.0 0 0)
  (Variables|Default|SetOriginalScale (Transformation|GetWorldScale _skeletalmesh))
  (bind _scale (Timeline|Timeline_0 PlayFromStart)
    (:Update
      (Transformation|SetWorldScale3D _skeletalmesh (* (Variables|Default|GetOriginalScale) (Math|Conversions|ToVector(Float) _scale))))))

(event EventTick
  (params (DeltaSeconds :type Float%20%28single-precision%29))
  (bind _returnvalue (Game|GetPlayerController 0))
  (bind _destinationactor (Variables|Default|GetDestinationActor))
  (Utilities|IsValid (Variables|Default|GetDestinationActor)
    (:Is%20Valid
      (Transformation|SetActorTransform (Class|KismetMathLibrary|TInterpto (Transformation|GetActorTransform) (Variables|Default|GetDestinationTransform) DeltaSeconds (Variables|Default|GetMovementSpeed)) false true)
      (if (< (Math|Vector|Distance(Vector) (Transformation|GetActorLocation) (.Location (Math|Transform|BreakTransform (Variables|Default|GetDestinationTransform)))) 15.0)
        (Pawn|UnPossess _returnvalue)
        (Actor|DestroyActor)
        (Pawn|Possess _returnvalue _destinationactor)
        (Variables|/Script/Engine.Actor|SetCustomTimeDilation _destinationactor 1.0)))))

(fn ConstructionScript)

(fn GiveDestination
  (params (destActor :type Pawn%20Object%20Reference))
  (bind _output_get (Variables|Default|SetDestinationActor destActor))
  (Variables|Default|SetDestinationTransform (Transformation|GetWorldTransform (Actor|GetComponentbyClass _output_get "/Script/Engine.CameraComponent")))
  (Development|PrintString "Destination found"))