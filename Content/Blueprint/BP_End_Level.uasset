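; Level exit actor that loads the next level once both the light and shadow characters stand in its capsule.
; Overlaps track the character count and which type is present, and disable death for characters while inside.
; Each change rebuilds dynamic materials to glow or displace per character and speeds up the skeletal mesh animation.
; At two characters, a one-shot delay fires the level-end call and opens NextSceneName, without rechecking occupancy.
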(event OnComponentBeginOverlap(Capsule)
  (params (OverlappedComponent :type Primitive%20Component%20Object%20Reference) (OtherActor :type Actor%20Object%20Reference) (OtherComp :type Primitive%20Component%20Object%20Reference) (OtherBodyIndex :type Integer) (bFromSweep :type Boolean) (SweepResult :type Hit%20Result%20Structure%20%28by%20ref%29))
  (bind _asthird_person_character (Utilities|Casting|CastToThirdPersonCharacter OtherActor))
  (Variables|/Game/ThirdPersonBP/Blueprints/ThirdPersonCharacter.ThirdPersonCharacter_C|SetallowDeath _asthird_person_character false)
  (bind _result (Math|Integer|IncrementInt (Variables|Default|GetCharacterCount))
    (:%20%20
      (bind _output_get (Variables|Default|SetCharacterCount _result))
      (Utilities|FlowControl|Sequence
        (:then_0
          (if (>= _output_get 2)
            (Utilities|FlowControl|DoOnce false
              (:Completed
                (Utilities|FlowControl|Delay 2.0)
                (Default|CallOnLevelEnd)
                (Game|OpenLevel(byName) (Utilities|String|StringToName (Variables|Default|GetNextSceneName)))))))
        (:then_1
          (if (Variables|/Game/ThirdPersonBP/Blueprints/ThirdPersonCharacter.ThirdPersonCharacter_C|GetIsLightChara _asthird_person_character)
            (Variables|Default|SetLightHere true)
            ;[1 1 1] SetLightMat
            (bind _returnvalue (Rendering|Material|CreateDynamicMaterialInstance (Variables|Default|GetSkeletalMesh) 1 "/Game/Geometry/Materials/MI_Light_Player.MI_Light_Player" "None" :!class /Script/Engine.PrimitiveComponent))
            (bind _returnvalue_2 (Rendering|Material|GetScalarParameterValue _returnvalue "EmissIntensity" :!class /Script/Engine.MaterialInstanceDynamic))
            (bind _output_get_2 (Variables|Default|SetEmiss_Instance _returnvalue))
            (Rendering|Material|SetScalarParameterValue _output_get_2 "EmissIntensity" (select (Variables|Default|GetLightHere) _returnvalue_2 0.2) :!class /Script/Engine.MaterialInstanceDynamic)
            (else
              (Variables|Default|SetShadowHere true)
              ;[1 1 1] SetShadowMat
              (bind _returnvalue_3 (Rendering|Material|CreateDynamicMaterialInstance (Variables|Default|GetSkeletalMesh) 0 "/Game/Geometry/Materials/MI_Dark_Player.MI_Dark_Player" "None" :!class /Script/Engine.PrimitiveComponent))
              (bind _output_get_3 (Variables|Default|SetEmiss_Instance2 _returnvalue_3))
              (Rendering|Material|SetScalarParameterValue _output_get_3 "EmissiveIntensity" (select (Variables|Default|GetShadowHere) 1e+04 0.0) :!class /Script/Engine.MaterialInstanceDynamic)
              (Rendering|Material|SetScalarParameterValue _output_get_3 "NoiseDispScale" (select (Variables|Default|GetShadowHere) 8.0 1.0) :!class /Script/Engine.MaterialInstanceDynamic))))
        (:then_2
          (Components|Timeline|SetPlayRate (Variables|Default|GetSkeletalMesh) (+ (* (Variables|Default|GetCharacterCount) 0.2) 0.1)))))))

(event OnComponentEndOverlap(Capsule)
  (params (OverlappedComponent :type Primitive%20Component%20Object%20Reference) (OtherActor :type Actor%20Object%20Reference) (OtherComp :type Primitive%20Component%20Object%20Reference) (OtherBodyIndex :type Integer))
  (bind _asthird_person_character (Utilities|Casting|CastToThirdPersonCharacter OtherActor))
  (Variables|/Game/ThirdPersonBP/Blueprints/ThirdPersonCharacter.ThirdPersonCharacter_C|SetallowDeath _asthird_person_character true)
  (bind _result (Math|Integer|DecrementInt (Variables|Default|GetCharacterCount))
    (:%20%20
      (Variables|Default|SetCharacterCount _result)
      (Utilities|FlowControl|Sequence
        (:then_0
          (if (Variables|/Game/ThirdPersonBP/Blueprints/ThirdPersonCharacter.ThirdPersonCharacter_C|GetIsLightChara _asthird_person_character)
            (Variables|Default|SetLightHere false)
            ;[1 1 1] SetLightMat
            (bind _returnvalue (Rendering|Material|CreateDynamicMaterialInstance (Variables|Default|GetSkeletalMesh) 1 "/Game/Geometry/Materials/MI_Light_Player.MI_Light_Player" "None" :!class /Script/Engine.PrimitiveComponent))
            (bind _returnvalue_2 (Rendering|Material|GetScalarParameterValue _returnvalue "EmissIntensity" :!class /Script/Engine.MaterialInstanceDynamic))
            (bind _output_get (Variables|Default|SetEmiss_Instance _returnvalue))
            (Rendering|Material|SetScalarParameterValue _output_get "EmissIntensity" (select (Variables|Default|GetLightHere) _returnvalue_2 0.2) :!class /Script/Engine.MaterialInstanceDynamic)
            (else
              (Variables|Default|SetShadowHere false)
              ;[1 1 1] SetShadowMat
              (bind _returnvalue_3 (Rendering|Material|CreateDynamicMaterialInstance (Variables|Default|GetSkeletalMesh) 0 "/Game/Geometry/Materials/MI_Dark_Player.MI_Dark_Player" "None" :!class /Script/Engine.PrimitiveComponent))
              (bind _output_get_2 (Variables|Default|SetEmiss_Instance2 _returnvalue_3))
              (Rendering|Material|SetScalarParameterValue _output_get_2 "EmissiveIntensity" (select (Variables|Default|GetShadowHere) 1e+04 0.0) :!class /Script/Engine.MaterialInstanceDynamic)
              (Rendering|Material|SetScalarParameterValue _output_get_2 "NoiseDispScale" (select (Variables|Default|GetShadowHere) 8.0 1.0) :!class /Script/Engine.MaterialInstanceDynamic))))
        (:then_1
          (Components|Timeline|SetPlayRate (Variables|Default|GetSkeletalMesh) (+ (* (Variables|Default|GetCharacterCount) 0.2) 0.1)))))))

(event EventBeginPlay
  (Utilities|FlowControl|Sequence
    (:then_0
      ;[1 1 1] SetLightMat
      (bind _returnvalue (Rendering|Material|CreateDynamicMaterialInstance (Variables|Default|GetSkeletalMesh) 1 "/Game/Geometry/Materials/MI_Light_Player.MI_Light_Player" "None" :!class /Script/Engine.PrimitiveComponent))
      (bind _returnvalue_2 (Rendering|Material|GetScalarParameterValue _returnvalue "EmissIntensity" :!class /Script/Engine.MaterialInstanceDynamic))
      (bind _output_get (Variables|Default|SetEmiss_Instance _returnvalue))
      (Rendering|Material|SetScalarParameterValue _output_get "EmissIntensity" (select (Variables|Default|GetLightHere) _returnvalue_2 0.2) :!class /Script/Engine.MaterialInstanceDynamic))
    (:then_1
      ;[1 1 1] SetShadowMat
      (bind _returnvalue_3 (Rendering|Material|CreateDynamicMaterialInstance (Variables|Default|GetSkeletalMesh) 0 "/Game/Geometry/Materials/MI_Dark_Player.MI_Dark_Player" "None" :!class /Script/Engine.PrimitiveComponent))
      (bind _output_get_2 (Variables|Default|SetEmiss_Instance2 _returnvalue_3))
      (Rendering|Material|SetScalarParameterValue _output_get_2 "EmissiveIntensity" (select (Variables|Default|GetShadowHere) 1e+04 0.0) :!class /Script/Engine.MaterialInstanceDynamic)
      (Rendering|Material|SetScalarParameterValue _output_get_2 "NoiseDispScale" (select (Variables|Default|GetShadowHere) 8.0 1.0) :!class /Script/Engine.MaterialInstanceDynamic))
    (:then_2
      (Components|Timeline|SetPlayRate (Variables|Default|GetSkeletalMesh) (+ (* (Variables|Default|GetCharacterCount) 0.2) 0.1)))))

(event Collision|EventActorBeginOverlap
  (params (OtherActor :type Actor%20Object%20Reference)))

(event EventTick
  (params (DeltaSeconds :type Float%20%28single-precision%29)))

(fn ConstructionScript)