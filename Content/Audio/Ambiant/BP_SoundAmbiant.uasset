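; BP_SoundAmbiant is an ambient sound Blueprint that switches its audio according to whether the possessed character is the light one.
; On BeginPlay it zeroes the PlayerIndex audio parameter and binds one handler to OnPlayerPossessed on the player's ThirdPersonCharacter and its OtherPawn.
; That handler sets PlayerIndex on the AudioComponent from IsPlayerLight.
; RefreshPlayerIndex is an empty stub.
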(event Custom|OnPlayerPossessed_Event_0
  (params (IsPlayerLight :type Boolean))
  (Effects|Components|ParticleSystem|SetIntParameter (Variables|Components|GetAudioComponent) "PlayerIndex" (Math|Integer|SelectInt 0 1 IsPlayerLight)))

(event EventBeginPlay
  (bind _asthird_person_character (Utilities|Casting|CastToThirdPersonCharacter (Game|GetPlayerCharacter 0)))
  (Effects|Components|ParticleSystem|SetIntParameter (Variables|Components|GetAudioComponent) "PlayerIndex" 0)
  (EventDispatchers|AssignOnPlayerPossessed _asthird_person_character (delegate Custom|OnPlayerPossessed_Event_0))
  (bind _asthird_person_character_2 (Utilities|Casting|CastToThirdPersonCharacter (Variables|/Game/ThirdPersonBP/Blueprints/ThirdPersonCharacter.ThirdPersonCharacter_C|GetOtherPawn _asthird_person_character)))
  (EventDispatchers|BindEventtoOnPlayerPossessed _asthird_person_character_2 (delegate Custom|OnPlayerPossessed_Event_0)))

(event EventTick
  (params (DeltaSeconds :type Float%20%28single-precision%29)))

(fn ConstructionScript)

(fn RefreshPlayerIndex
  (params (IsLight :type Boolean)))